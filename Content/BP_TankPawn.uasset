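; Tank pawn Blueprint that handles the tank's UI: health bar, main menu toggle and game-over screen.
; On BeginPlay it caches the WBP_HP from its HealthBar widget component and copies in the HealthComponent's health state, refreshing it on each TakeDamageEvent.
; The P key uses a FlipFlop to show or remove the main menu through AWidgetHUD.
; GameOverEvent creates the game-over widget and adds it to the viewport.
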(event `Key|P`
  (params (Key :type "Key Structure"))
  ;[1 1 1] Menu bar
  (:`Pressed`
    (bind _asawidget_hud (cast `AWidgetHUD` (`PlayerController.GetHUD` (`GameplayStatics.GetPlayerController` 0))))
    (`/Engine/EditorBlueprintResources/StandardMacros.FlipFlop`
      (:`A`
        (`AWidgetHUD.UseWidget` _asawidget_hud "MainMenu" true 0))
      (:`B`
        (`AWidgetHUD.RemoveCurrentWidgetFromViewport` _asawidget_hud)))))

(event `self.ReceiveBeginPlay`
  ;[1 1 1] Когда игра стартует появляется виджет Health Bar
  (bind _aswbp_hp (cast `/Game/UI/Health_/WBP_HP` (`WidgetComponent.GetWidget` (`self.HealthBar`))))
  (bind _output_get (set `self.HealthBP` _aswbp_hp))
  (set `/Game/UI/Health_/WBP_HP.HealthState` (`HealthComponent.GetHealthState` (`self.HealthComponent`)) _output_get))

(event `self.TakeDamageEvent`
  ;[1 1 1] Когда получаем урон Health Bar Уменьшается
  (set `/Game/UI/Health_/WBP_HP.HealthState` (`HealthComponent.GetHealthState` (`self.HealthComponent`)) (`self.HealthBP`)))

(event `self.GameOverEvent`
  (bind _returnvalue (`|CreateWidget` "/Game/UI/Menu/GameOverWBP.GameOverWBP_C"))
  (`UserWidget.AddToViewport` _returnvalue 0))

(fn `UserConstructionScript`)