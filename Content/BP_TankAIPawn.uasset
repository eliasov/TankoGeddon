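; BP_TankAIPawn is an AI tank pawn Blueprint that shows the tank's health on a health bar widget.
; On BeginPlay it casts the HealthBar component's widget to WBP_HP, stores it and sets its HealthState from HealthComponent.
; TakeDamageEvent pushes the current health state to that widget again, so the bar updates on damage events instead of every tick.
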(event `self.ReceiveBeginPlay`
  ;[1 1 1] Когда игра стартует появляется виджет Health Bar
  (bind _aswbp_hp (cast `/Game/UI/Health_/WBP_HP` (`WidgetComponent.GetWidget` (`self.HealthBar`))))
  (bind _output_get (set `self.HealthBP` _aswbp_hp))
  (set `/Game/UI/Health_/WBP_HP.HealthState` (`HealthComponent.GetHealthState` (`self.HealthComponent`)) _output_get))

(event `self.TakeDamageEvent`
  ;[1 1 1] Когда получаем урон Health Bar Уменьшается
  (set `/Game/UI/Health_/WBP_HP.HealthState` (`HealthComponent.GetHealthState` (`self.HealthComponent`)) (`self.HealthBP`)))

(fn `UserConstructionScript`)